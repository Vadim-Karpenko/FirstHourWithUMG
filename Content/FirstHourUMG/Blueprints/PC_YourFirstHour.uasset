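; PC_YourFirstHour is a player controller that toggles a pause menu when the Pause input action is pressed.
; Opening creates UMG_MainMenu, pauses the game, shows the cursor and switches to Game and UI input; closing removes the widget and reverses those changes.
; The stored widget reference serves as the toggle state.
; Each toggle also tells Character_FirstHourUMG to turn its UI off or back on.
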(event Input|ActionEvents|InputActionPause
  (params (Key :type Key%20Structure :default "None"))
  (bind _returnvalue (Game|GetPlayerController 0))
  (bind _returnvalue_2 (Game|GetPlayerCharacter 0))
  (:Pressed
    (Utilities|IsValid (Variables|Default|GetPauseUIRef)
      (:Is%20Valid
        ;[1 1 1] Unpause
        (Widget|RemovefromParent (Variables|Default|GetPauseUIRef))
        (Variables|Default|SetPauseUIRef 0)
        (Input|SetInputModeGameOnly (Game|GetPlayerController 0))
        (Variables|Default|SetbShowMouseCursor false)
        (Game|SetGamePaused false)
        (bind _ascharacter_first_hour_umg (Utilities|Casting|CastToCharacter_FirstHourUMG _returnvalue_2))
        (Default|TurnUIon _ascharacter_first_hour_umg))
      (:Is%20Not%20Valid
        ;[1 1 1] Show pause
        (bind _returnvalue_3 (UserInterface|CreateWidget "/Game/FirstHourUMG/Widgets/UMG_MainMenu.UMG_MainMenu_C" _returnvalue))
        (bind _output_get (Variables|Default|SetPauseUIRef _returnvalue_3))
        (UserInterface|Viewport|AddtoViewport _output_get 0)
        (Input|SetInputModeGameandUI _returnvalue 0 "DoNotLock" true)
        (Variables|Default|SetbShowMouseCursor true)
        (Game|SetGamePaused true)
        (bind _ascharacter_first_hour_umg_2 (Utilities|Casting|CastToCharacter_FirstHourUMG _returnvalue_2))
        (Default|TurnUIOff _ascharacter_first_hour_umg_2)))))

(fn ConstructionScript)